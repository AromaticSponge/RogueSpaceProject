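; Game mode for Rogue Space that drives the game loop through menu, pre-game upgrade, base and boss phases.
; E_Init sets up the player controller, then E_GameLogic switches on GameplayState and re-calls itself on transitions.
; The menu shows the master HUD and auto-advances after a temporary delay.
; Base phase runs a timer into boss phase, which immediately loops back to base; boss spawning is an empty stub.
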(event `E_Init`
  (`self.F_SetupPlayer`)
  (`self.E_GameLogic`))

(event `E_GameLogic`
  (bind _hud (`self.HUD`))
  (switch `/Game/Blueprint/Systems/GamePlayState` (`self.GameplayState`)
    (:`NewEnumerator0`
      (`/Engine/EditorBlueprintResources/StandardMacros.IsValid` (`self.HUD`)
        (:`Is Valid`
          _)
        (:`Is Not Valid`
          (bind _returnvalue (`|CreateWidget` "/Game/UMG/MasterHUD.MasterHUD_C"))
          (set `self.HUD` _returnvalue)))
      (`UserWidget.AddToViewport` _hud 0)
      ;[1 1 1] temporary, will trigger when the player moves into the game
      (`KismetSystemLibrary.Delay` 2.0)
      (`/Game/UMG/MasterHUD.E_TitleExitAnim` _hud)
      (set `self.GameplayState` "NewEnumerator1")
      (`self.E_GameLogic`))
    (:`NewEnumerator1`
      (`self.F_PreGamePhase`))
    (:`NewEnumerator2`
      (`self.F_BasePhase`))
    (:`NewEnumerator3`
      (`self.F_BossPhase`))))

(event `E_StartGameTimer`
  (bind _returnvalue (`KismetSystemLibrary.K2_SetTimerDelegate` (delegate `E_BossPhase`) (`self.Phase1Length`)))
  (set `self.GameTimer` _returnvalue))

(event `E_BossPhase`
  (set `self.GameplayState` "NewEnumerator3")
  (`self.E_GameLogic`))

(fn `F_BasePhase`
  (`self.E_StartGameTimer`))

(fn `F_BossPhase`
  (`KismetSystemLibrary.K2_ClearAndInvalidateTimerHandle` (`self.GameTimer`))
  (`self.F_SpawnBoss`)
  (`/Game/UMG/MasterHUD.E_BossTextAnim` (`self.HUD`))
  (set `self.GameplayState` "NewEnumerator2")
  (`self.E_GameLogic`))

(fn `F_PreGamePhase`
  (`/Game/Blueprint/Player/RogueSpacePlayerController.F_ReadyToPlay` (`self.PlayerController`))
  (set `self.GameplayState` "NewEnumerator2")
  (`self.E_GameLogic`))

(fn `F_SetupPlayer`
  (bind _asrogue_space_player_controller (cast `/Game/Blueprint/Player/RogueSpacePlayerController` (`GameplayStatics.GetPlayerController` 0)))
  (bind _output_get (set `self.PlayerController` _asrogue_space_player_controller))
  (`/Game/Blueprint/Player/RogueSpacePlayerController.E_Init` _output_get))

(fn `F_SpawnBoss`
  ;[1 1 1] Spawn boss and bind event to its death to advance to next level
)

(fn `UserConstructionScript`)