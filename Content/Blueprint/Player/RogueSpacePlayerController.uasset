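; Player controller that spawns the player ship, manages its possession and forwards movement input to it.
; On init it replaces the default pawn with a scaled-down ship at the first PlayerSpawn, leaves it unpossessed, sets the view to MainCamera and shows the cursor.
; A ready-to-play function possesses the ship and restores that camera, while exit-play unpossesses.
; Movement axis input reaches the ship through an interface message only while a pawn is controlled.
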(event `E_Init`
  (`self.F_SpawnPlayer`)
  (`self.F_SetCamera`)
  (set `self.bShowMouseCursor` true))

(event `InputAxis|Movement`
  (params (AxisValue :type "Float (single-precision)"))
  (`/Engine/EditorBlueprintResources/StandardMacros.IsValid` (`self.K2_GetPawn`)
    (:`Is Valid`
      (message `/Game/Blueprint/Interfaces/PlayerControlInterface.IMovement` (`self.PlayerShip`) AxisValue))))

(fn `F_ExitPlay`
  (`self.UnPossess`))

(fn `F_ReadyToPlay`
  (`self.Possess` (`self.PlayerShip`))
  (`self.F_SetCamera`))

(fn `F_SetCamera`
  (locals (TempCamera :type "CameraActor Object Reference"))
  (bind _outactors (`GameplayStatics.GetAllActorsOfClass` "/Script/Engine.CameraActor"))
  (for _array_element _outactors
    (if (`KismetStringLibrary.EqualEqual_StrStr` (`KismetSystemLibrary.GetObjectName` _array_element) "MainCamera")
      (set `local.TempCamera` _array_element)
      (break)))
  (`self.SetViewTargetWithBlend` (`local.TempCamera`)))

(fn `F_SpawnPlayer`
  ;[1 1 1] Destroy the pawn UE4 spawns and set up the player ship
  (`self.K2_DestroyActor` (`self.K2_GetPawn`))
  (bind _outactors (`GameplayStatics.GetAllActorsOfClass` "/Game/Blueprint/Player/PlayerSpawn.PlayerSpawn_C"))
  (bind (_returnvalue_location _returnvalue_rotation) (`KismetMathLibrary.BreakTransform` (`self.GetTransform` (`|GetArrayItem` _outactors))))
  (bind _returnvalue (`|SpawnActorFromClass` "/Game/Blueprint/Player/PlayerShip.PlayerShip_C" (`KismetMathLibrary.MakeTransform` _returnvalue_location _returnvalue_rotation (0.05 0.05 0.05)) "AlwaysSpawn" "OverrideRootScale" null self null))
  (bind _output_get (set `self.PlayerShip` _returnvalue))
  (`/Game/Blueprint/Player/BaseShipClass.E_Init` _output_get)
  (`self.F_ExitPlay`))

(fn `UserConstructionScript`)