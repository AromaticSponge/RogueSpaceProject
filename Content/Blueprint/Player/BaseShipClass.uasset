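; Base player ship class that moves a physics mesh with debug WASD input, slows it down and tilts it sideways.
; Axis events apply velocity-change impulses and set a Moving flag.
; E_Init starts a looping timer, used instead of Tick, that divides velocity for deceleration and interpolates rotation by AnimationState.
; F_SetAnimType derives that state from Y velocity, but nothing in this file calls it.
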(event `E_Init`
  ;[1 1 1] Initialisation
  (`self.E_SetUpTimer`))

(event `E_MoveUp`
  (params (Axis :type "Float (double-precision)"))
  ;[1 1 1] Used for moving with wasd, DEBUG
  (if (!= Axis 0.0)
    (set `self.Moving` true)
    (else
      (set `self.Moving` false)))
  (`PrimitiveComponent.AddImpulse` (`self.ShipMesh`) (`KismetMathLibrary.MakeVector` (* Axis (`self.Speed`))) "None" true))

(event `EMoveLeft`
  (params (Axis :type "Float (double-precision)"))
  ;[1 1 1] Used for moving with wasd, DEBUG
  (if (!= Axis 0.0)
    (set `self.Moving` true)
    (else
      (set `self.Moving` false)))
  (`PrimitiveComponent.AddImpulse` (`self.ShipMesh`) (`KismetMathLibrary.MakeVector` 0.0 (* Axis (`self.Speed`))) "None" true))

(event `E_SetUpTimer`
  ;[1 1 1] Timer
  (`KismetSystemLibrary.K2_SetTimerDelegate` (delegate `E_TImerActions`) 0.05 true))

(event `E_TImerActions`
  ;[1 1 1] Timer
  (`self.E_Deccelarion`)
  (`self.E_TiltAnimation`))

(event `E_Deccelarion`
  (bind _decceleration (`self.Decceleration`))
  (bind _shipmesh (`self.ShipMesh`))
  (bind (_returnvalue_x _returnvalue_y _returnvalue_z) (`KismetMathLibrary.BreakVector` (`SceneComponent.GetComponentVelocity` _shipmesh)))
  ;[1 1 1] Used for decceleration
  (`PrimitiveComponent.SetPhysicsLinearVelocity` _shipmesh (`KismetMathLibrary.MakeVector` (/ _returnvalue_x _decceleration) (/ _returnvalue_y _decceleration) (/ _returnvalue_z _decceleration)) false "None"))

(event `E_TiltAnimation`
  (bind _shipmesh (`self.ShipMesh`))
  (bind _returnvalue (`SceneComponent.K2_GetComponentRotation` _shipmesh))
  ;[1 1 1] Tilt Animation
  (switch `/Game/Blueprint/Player/AnimationStates` (`self.AnimationState`)
    (:`NewEnumerator0`
      (`SceneComponent.K2_SetWorldRotation` _shipmesh (`KismetMathLibrary.RInterpTo_Constant` _returnvalue (struct) 0.05 2.0) false true))
    (:`NewEnumerator1`
      (`SceneComponent.K2_SetWorldRotation` _shipmesh (`KismetMathLibrary.RInterpTo_Constant` _returnvalue (struct :`Roll` 30.0) 0.005 2.0) false true))
    (:`NewEnumerator2`
      (`SceneComponent.K2_SetWorldRotation` _shipmesh (`KismetMathLibrary.RInterpTo_Constant` _returnvalue (struct :`Roll` -30.0) 0.005 2.0) false true))))

(fn `F_SetAnimType`
  (bind (_returnvalue_x _returnvalue_y) (`KismetMathLibrary.BreakVector` (`SceneComponent.GetComponentVelocity` (`self.ShipMesh`))))
  (if (> _returnvalue_y 0.0)
    (set `self.AnimationState` "NewEnumerator1")
    (elif (< _returnvalue_y 0.0)
      (set `self.AnimationState` "NewEnumerator2")
      (else
        (set `self.AnimationState` "NewEnumerator0"))))
  (return))

(fn `UserConstructionScript`)