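; PlayerShip is the player-controlled ship Blueprint, which moves by physics impulses toward the cursor.
; While the Movement axis is positive, a Visibility trace under the cursor yields a target, and the mesh receives an impulse scaled by Speed and the unnormalized offset, so distant targets push harder.
; A hit also updates the animation type; releasing input resets movement and animation state.
; MoveUp and MoveLeft axes forward to events defined outside these graphs.
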(event `InputAxis|MoveUp`
  (params (AxisValue :type "Float (single-precision)"))
  (`self.E_MoveUp` AxisValue))

(event `InputAxis|MoveLeft`
  (params (AxisValue :type "Float (single-precision)"))
  (`self.EMoveLeft` AxisValue))

(event `InputAxis|Movement`
  (params (AxisValue :type "Float (single-precision)"))
  (bind _shipmesh (`self.ShipMesh`))
  (bind (_hitresult _returnvalue) (`PlayerController.GetHitResultUnderCursorByChannel` (`self.PlayerController`) "TraceTypeQuery1" true))
  ;[1 1 1] Click / touch to move
  (if (> AxisValue 0.0)
    (set `self.Moving` true)
    (if _returnvalue
      (`PrimitiveComponent.AddImpulse` _shipmesh (* (- (`.Location` (`GameplayStatics.BreakHitResult` _hitresult)) (`SceneComponent.K2_GetComponentLocation` _shipmesh)) (`self.Speed`)) "None" false)
      (`self.F_SetAnimType`))
    (else
      (set `self.Moving` false)
      (set `self.AnimationState` "NewEnumerator0"))))

(fn `UserConstructionScript`
  (`parent.UserConstructionScript`))